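; General_Helpers is a Blueprint helper set of debug print functions for logging the status of named system events on screen.
; BeginEventPrint, SuccessPrint and ErrorPrint each format the system and event names into a dashed banner and pass it to PrintString.
; Each status has its own text color: cyan for playing, green for success and red for error, which also includes a response message.
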(fn ErrorPrint
  (params (system :type String) (%20event%20 :type String) (%20response%20 :type String))
  (Development|PrintString 0 (Utilities|String|ToString(Text) (Utilities|Text|FormatText "---------------------- 
( {system} ): { event } Event Error. 
Response: { response } 
---------------------- 
" system %20event%20 %20response%20)) true true "(R=1.000000,G=0.042732,B=0.000000,A=1.000000)"))

(fn SuccessPrint
  (params (system :type String) (%20event%20 :type String))
  (Development|PrintString 0 (Utilities|String|ToString(Text) (Utilities|Text|FormatText "---------------------- 
( {system} ): { event } Event Success 
---------------------- 
" system %20event%20)) true true "(R=0.138322,G=1.000000,B=0.000000,A=1.000000)"))

(fn BeginEventPrint
  (params (system :type String) (%20event%20 :type String))
  (Development|PrintString 0 (Utilities|String|ToString(Text) (Utilities|Text|FormatText "---------------------- 
( {system} ): { event } Event Playing 
---------------------- 
" system %20event%20)) true true "(R=0.000000,G=1.000000,B=0.921138,A=1.000000)"))